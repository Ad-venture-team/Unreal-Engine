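; BP_Mine is an interactable mine building that opens its own UI_Mine menu.
; A sphere's overlap events show and hide a Widget component as anything enters or leaves, with no filter on the overlapping actor.
; The menu is created and cached on BeginPlay, then Interact adds it to the viewport, switches player 0 to UI-only input and shows the mouse cursor.
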(event `self.Sphere.OnComponentBeginOverlap`
  (params (OverlappedComponent :type "PrimitiveComponent Object Reference") (OtherActor :type "Actor Object Reference") (OtherComp :type "PrimitiveComponent Object Reference") (OtherBodyIndex :type Integer) (bFromSweep :type Boolean) (SweepResult :type "HitResult Structure (by ref)"))
  (`SceneComponent.SetVisibility` (`self.Widget`) true false))

(event `self.Sphere.OnComponentEndOverlap`
  (params (OverlappedComponent :type "PrimitiveComponent Object Reference") (OtherActor :type "Actor Object Reference") (OtherComp :type "PrimitiveComponent Object Reference") (OtherBodyIndex :type Integer))
  (`SceneComponent.SetVisibility` (`self.Widget`) false false))

(event `self.ReceiveBeginPlay`
  (bind _returnvalue (`|CreateWidget` "/Game/UI/UI_Mine.UI_Mine_C"))
  (set `self.MineUI` _returnvalue))

(event `/Game/Character/Interact_Interface.Interact`
  (bind _returnvalue (`GameplayStatics.GetPlayerController` 0))
  (bind _mineui (`self.MineUI`))
  (`UserWidget.AddToViewport` _mineui 0)
  (`WidgetBlueprintLibrary.SetInputMode_UIOnlyEx` _returnvalue _mineui)
  (set `PlayerController.bShowMouseCursor` true _returnvalue))

(fn `UserConstructionScript`)