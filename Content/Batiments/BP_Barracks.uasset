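; BP_Barracks is a barracks building that the player can interact with to open its UI.
; A sphere overlap shows a widget component while something is in range and hides it on exit, with no filter on the overlapping actor.
; BeginPlay creates the UI_Barracks widget once, and Interact adds it to the viewport, switches input to UI only and shows the mouse cursor.
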(event `self.Sphere.OnComponentBeginOverlap`
  (params (OverlappedComponent :type "PrimitiveComponent Object Reference") (OtherActor :type "Actor Object Reference") (OtherComp :type "PrimitiveComponent Object Reference") (OtherBodyIndex :type Integer) (bFromSweep :type Boolean) (SweepResult :type "HitResult Structure (by ref)"))
  (`SceneComponent.SetVisibility` (`self.Widget`) true false))

(event `self.Sphere.OnComponentEndOverlap`
  (params (OverlappedComponent :type "PrimitiveComponent Object Reference") (OtherActor :type "Actor Object Reference") (OtherComp :type "PrimitiveComponent Object Reference") (OtherBodyIndex :type Integer))
  (`SceneComponent.SetVisibility` (`self.Widget`) false false))

(event `self.ReceiveBeginPlay`
  (bind _returnvalue (`|CreateWidget` "/Game/Batiments/UI_Barracks.UI_Barracks_C"))
  (set `self.BarrackUI` _returnvalue))

(event `/Game/Character/Interact_Interface.Interact`
  (bind _returnvalue (`GameplayStatics.GetPlayerController` 0))
  (bind _barrackui (`self.BarrackUI`))
  (`UserWidget.AddToViewport` _barrackui 0)
  (`WidgetBlueprintLibrary.SetInputMode_UIOnlyEx` _returnvalue _barrackui)
  (set `PlayerController.bShowMouseCursor` true _returnvalue))

(fn `UserConstructionScript`)